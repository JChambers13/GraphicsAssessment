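; BP_CameraSwitch is a proximity-triggered actor that lets the player cycle through security-style camera views and springs an AI enemy spawn.
; Overlap enables input, and Tick responds to C by blending the view through the Cameras array and back to the pawn, using a short delayed flag as debounce.
; Reaching the fifth step spawns BP_AIEntity at SpawnPoint once, briefly disabling input during the spawn.
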(event `self.ReceiveBeginPlay`
  (set `self.PlayerController` (`GameplayStatics.GetPlayerController` 0))
  (set `self.PlayerPawn` (`GameplayStatics.GetPlayerPawn` 0))
  (set `self.One` 1)
  (set `self.EnemySpawned` false))

(event `Key|C`
  (params (Key :type "Key Structure"))
  (:`Pressed`
    (set `self.CPressed` true))
  (:`Released`
    (set `self.CPressed` false)))

(event `self.ReceiveActorBeginOverlap`
  (params (OtherActor :type "Actor Object Reference"))
  ; Determine if player is near the generator. If player is near, enable input
  (set `self.PlayerNear` true)
  (`self.EnableInput` (`GameplayStatics.GetPlayerController` 0)))

(event `Spawn Enemy`
  (bind _playercontroller (`self.PlayerController`))
  (`|SpawnActorFromClass` "/Game/MyContent/MyBlueprints/BP_AIEntity.BP_AIEntity_C" (`SceneComponent.K2_GetComponentToWorld` (`Actor.RootComponent` (`self.SpawnPoint`))) "AlwaysSpawn" "MultiplyWithRoot" null null)
  (set `self.CPressed` false)
  (`self.DisableInput` _playercontroller)
  (`KismetSystemLibrary.Delay` 1.0)
  (set `self.EnemySpawned` true)
  (`self.EnableInput` _playercontroller))

(event `self.ReceiveActorEndOverlap`
  (params (OtherActor :type "Actor Object Reference"))
  ; Determine if player is near the generator. If player is near, enable input
  (set `self.PlayerNear` false)
  (`self.DisableInput` (`GameplayStatics.GetPlayerController` 0)))

(event `self.ReceiveTick`
  (params (DeltaSeconds :type "Float (single-precision)"))
  (if (and (`self.PlayerNear`) (`self.CPressed`) (not (`self.JustSwitched`)))
    (`KismetSystemLibrary.PrintString` "new cam")
    (set `self.CurrentCam` (+ (`self.CurrentCam`) 1))
    ; False if current cam > length
    (if (< (`self.CurrentCam`) (`KismetArrayLibrary.Array_Length` (`self.Cameras`)))
      (`PlayerController.SetViewTargetWithBlend` (`self.PlayerController`) (`|GetArrayItem` (`self.Cameras`) (- (`self.CurrentCam`) 1)) 0.2 "VTBlend_Linear" 0.0 false)
      (set `self.JustSwitched` true)
      (if (and (== (`self.CurrentCam`) 5) (not (`self.EnemySpawned`)))
        (`self.Spawn Enemy`))
      (else
        (set `self.CurrentCam` 0)
        (`PlayerController.SetViewTargetWithBlend` (`self.PlayerController`) (`self.PlayerPawn`) 0.2 "VTBlend_Linear" 0.0 false)
        (set `self.JustSwitched` true)))
    (elif (`self.JustSwitched`)
      (`KismetSystemLibrary.Delay` 0.2)
      (set `self.JustSwitched` false))))

(fn `UserConstructionScript`)