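; Sliding door actor that moves itself open when an actor begins overlapping it and back closed when the overlap ends.
; BeginPlay stores the starting location as closed and derives the open location from a fixed world-space Y offset.
; Two separate timelines, each started with Play rather than Play from Start, lerp the whole actor between those points without sweeping.
; Overlap events do not filter which actor triggers them.
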(event `self.ReceiveBeginPlay`
  (bind _output_get (set `self.Closed Location` (`self.K2_GetActorLocation`)))
  (set `self.Open Location` (+ _output_get (0.0 300.0 0.0))))

(event `self.ReceiveActorBeginOverlap`
  (params (OtherActor :type "Actor Object Reference"))
  (bind (_direction _door_open) (`Timeline|Timeline`)
    (:`Update`
      (`self.K2_SetActorLocation` (`KismetMathLibrary.VLerp` (`self.Closed Location`) (`self.Open Location`) _door_open)))))

(event `self.ReceiveActorEndOverlap`
  (params (OtherActor :type "Actor Object Reference"))
  (bind (_direction _newtrack_0) (`Timeline|Timeline_0`)
    (:`Update`
      (`self.K2_SetActorLocation` (`KismetMathLibrary.VLerp` (`self.Open Location`) (`self.Closed Location`) _newtrack_0)))))

(fn `UserConstructionScript`)