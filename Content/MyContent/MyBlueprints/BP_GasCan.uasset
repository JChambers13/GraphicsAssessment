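; BP_GasCan is a gas can pickup that the player collects by pressing L while nearby.
; Overlap events toggle the actor's input and a proximity flag, while Tick polls that flag and the key state.
; If no can is already carried, CanID selects one of four generator-can flags to set in the BP_Global game instance, along with PlayerHasCan, then the actor destroys itself.
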(event `self.ReceiveTick`
  (params (DeltaSeconds :type "Float (single-precision)"))
  (bind _asbp_global (cast `/Game/MyContent/MyBlueprints/BP_Global` (`GameplayStatics.GetGameInstance`)))
  ; Check if gas can should be picked up
  (if (and (`self.L Pressed`) (`self.Player Near`) (not (`/Game/MyContent/MyBlueprints/BP_Global.PlayerHasCan` _asbp_global)))
    ; Pick up gas can
    (bind _asbp_global_2 (cast `/Game/MyContent/MyBlueprints/BP_Global` (`GameplayStatics.GetGameInstance`)))
    (switch `int` (`self.CanID`)
      (:`0`
        (set `/Game/MyContent/MyBlueprints/BP_Global.Gen1Can` true _asbp_global_2))
      (:`1`
        (set `/Game/MyContent/MyBlueprints/BP_Global.Gen2Can` true _asbp_global_2))
      (:`2`
        (set `/Game/MyContent/MyBlueprints/BP_Global.Gen3Can` true _asbp_global_2))
      (:`3`
        (set `/Game/MyContent/MyBlueprints/BP_Global.Gen4Can` true _asbp_global_2)))
    (set `/Game/MyContent/MyBlueprints/BP_Global.PlayerHasCan` true _asbp_global_2)
    (`self.K2_DestroyActor`)))

(event `self.ReceiveActorBeginOverlap`
  (params (OtherActor :type "Actor Object Reference"))
  ; Enable/Disable Player Input + Check if player is nearby
  (`self.EnableInput` (`GameplayStatics.GetPlayerController` 0))
  (set `self.Player Near` true))

(event `self.ReceiveActorEndOverlap`
  (params (OtherActor :type "Actor Object Reference"))
  ; Enable/Disable Player Input + Check if player is nearby
  (`self.DisableInput` (`GameplayStatics.GetPlayerController` 0))
  (set `self.Player Near` false))

(event `Key|L`
  (params (Key :type "Key Structure"))
  ; Set L Pressed
  (:`Pressed`
    (set `self.L Pressed` true))
  (:`Released`
    (set `self.L Pressed` false)))

(fn `UserConstructionScript`)