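; BP_DoorLight is an indicator light that glows once the generator matching its GeneratorID is on.
; BeginPlay puts a dynamic material instance on the Sphere.
; Tick polls one of four generator flags (Gen1 to Gen4) in the BP_Global game instance, then raises the Emission parameter once.
; Nothing switches the light back off, and Tick prints debug strings, including the generator state every frame.
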(event `self.ReceiveTick`
  (params (DeltaSeconds :type "Float (single-precision)"))
  (`|ExecutionSequence`
    (:`then_0`
      (`KismetSystemLibrary.PrintString` (`KismetStringLibrary.Conv_BoolToString` (`self.GeneratorOn`)))
      (bind _asbp_global (cast `/Game/MyContent/MyBlueprints/BP_Global` (`GameplayStatics.GetGameInstance`)))
      (switch `int` (`self.GeneratorID`)
        (:`0`
          (if (`/Game/MyContent/MyBlueprints/BP_Global.Gen1` _asbp_global)
            (set `self.GeneratorOn` true)))
        (:`1`
          (if (`/Game/MyContent/MyBlueprints/BP_Global.Gen2` _asbp_global)
            (set `self.GeneratorOn` true)))
        (:`2`
          (if (`/Game/MyContent/MyBlueprints/BP_Global.Gen3` _asbp_global)
            (set `self.GeneratorOn` true)))
        (:`3`
          (if (`/Game/MyContent/MyBlueprints/BP_Global.Gen4` _asbp_global)
            (set `self.GeneratorOn` true)))))
    (:`then_1`
      (if (and (not (`self.Light On`)) (`self.GeneratorOn`))
        (`KismetSystemLibrary.PrintString` "Hello")
        (`MaterialInstanceDynamic.SetScalarParameterValue` (`self.Light`) "Emission" 100.0)
        (set `self.Light On` true)))))

(event `self.ReceiveBeginPlay`
  (bind _returnvalue (`PrimitiveComponent.CreateDynamicMaterialInstance` (`self.Sphere`) 0 null "None"))
  (bind _output_get (set `self.Light` _returnvalue))
  (`PrimitiveComponent.SetMaterial` (`self.Sphere`) 0 _output_get)
  (set `self.Light On` false))

(fn `UserConstructionScript`)