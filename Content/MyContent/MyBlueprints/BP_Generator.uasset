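; BP_Generator is an interactable generator, identified by GeneratorID, that the player activates with G once its matching can is collected.
; Tick polls BP_Global in the game instance for that can, and overlap events toggle proximity and input.
; Activation turns a dynamic fuel-light material green, marks the generator completed, increments the global used count, clears the carried-can flag and sets that generator's global flag.
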(event `self.ReceiveTick`
  (params (DeltaSeconds :type "Float (single-precision)"))
  (`|ExecutionSequence`
    (:`then_0`
      ; Check if the can for this generator has been collected. Each generator is handled seperately through the Switch
      (bind _asbp_global (cast `/Game/MyContent/MyBlueprints/BP_Global` (`GameplayStatics.GetGameInstance`)))
      (switch `int` (`self.GeneratorID`)
        (:`0`
          (if (`/Game/MyContent/MyBlueprints/BP_Global.Gen1Can` _asbp_global)
            (set `self.Can Collected` true)))
        (:`1`
          (if (`/Game/MyContent/MyBlueprints/BP_Global.Gen2Can` _asbp_global)
            (set `self.Can Collected` true)))
        (:`2`
          (if (`/Game/MyContent/MyBlueprints/BP_Global.Gen3Can` _asbp_global)
            (set `self.Can Collected` true)))
        (:`3`
          (if (`/Game/MyContent/MyBlueprints/BP_Global.Gen4Can` _asbp_global)
            (set `self.Can Collected` true)))))
    (:`then_1`
      ; Handle generator being turned on
      (if (and (not (`self.Completed`)) (`self.PlayerNear`) (`self.G Presssed`) (`self.Can Collected`))
        (`MaterialInstanceDynamic.SetVectorParameterValue` (`self.FuelLightVar`) "Colour" (struct :`G` 1.0 :`A` 1.0))
        (set `self.Completed` true)
        (bind _asbp_global_2 (cast `/Game/MyContent/MyBlueprints/BP_Global` (`GameplayStatics.GetGameInstance`)))
        (bind _result (`/Engine/EditorBlueprintResources/StandardMacros.IncrementInt` (`/Game/MyContent/MyBlueprints/BP_Global.GensUsed` _asbp_global_2))
          (:`  `
            (set `/Game/MyContent/MyBlueprints/BP_Global.GensUsed` _result _asbp_global_2)
            (set `/Game/MyContent/MyBlueprints/BP_Global.PlayerHasCan` false _asbp_global_2)
            (bind _asbp_global_3 (cast `/Game/MyContent/MyBlueprints/BP_Global` (`GameplayStatics.GetGameInstance`)))
            (switch `int` (`self.GeneratorID`)
              (:`0`
                (set `/Game/MyContent/MyBlueprints/BP_Global.Gen1` true _asbp_global_3))
              (:`1`
                (set `/Game/MyContent/MyBlueprints/BP_Global.Gen2` true _asbp_global_3))
              (:`2`
                (set `/Game/MyContent/MyBlueprints/BP_Global.Gen3` true _asbp_global_3))
              (:`3`
                (set `/Game/MyContent/MyBlueprints/BP_Global.Gen4` true _asbp_global_3)))))))))

(event `Key|G`
  (params (Key :type "Key Structure"))
  ; Check if G is being pressed. This is only triggered when player is nearby
  (:`Pressed`
    (set `self.G Presssed` true))
  (:`Released`
    (set `self.G Presssed` false)))

(event `self.ReceiveActorBeginOverlap`
  (params (OtherActor :type "Actor Object Reference"))
  ; Determine if player is near the generator. If player is near, enable input
  (set `self.PlayerNear` true)
  (`self.EnableInput` (`GameplayStatics.GetPlayerController` 0)))

(event `self.ReceiveBeginPlay`
  (bind _generator_model (`self.Generator-model`))
  (bind _fuellightvar (`self.FuelLightVar`))
  ; Create dynamic material instance. This allows the fuel light to turn green when the generator is activated
  (bind _returnvalue (`PrimitiveComponent.CreateDynamicMaterialInstance` (`self.Generator-model`) 4 "/Game/MyContent/MyMaterials/M_FuelLight_Inst.M_FuelLight_Inst" "None"))
  (set `self.FuelLightVar` _returnvalue)
  (`PrimitiveComponent.SetMaterial` _generator_model 4 _fuellightvar)
  (`PrimitiveComponent.SetMaterial` _generator_model 5 _fuellightvar))

(event `self.ReceiveActorEndOverlap`
  (params (OtherActor :type "Actor Object Reference"))
  ; Determine if player is near the generator. If player is near, enable input
  (set `self.PlayerNear` false)
  (`self.DisableInput` (`GameplayStatics.GetPlayerController` 0)))

(fn `UserConstructionScript`)