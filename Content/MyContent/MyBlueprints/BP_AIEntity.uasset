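; AI enemy that wanders between the level's TargetPoints and chases the player on sight.
; After a brief spawn pause, Tick issues AIMoveTo toward either a random point or the player controller.
; Pawn sensing starts the chase, which reverts to wandering after two seconds without a sighting.
; The attack on reaching the player is a placeholder delay and print, and FollowPlayer is not called in this graph.
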(event `self.PawnSensing.OnSeePawn`
  (params (Pawn :type "Pawn Object Reference"))
  ; This is triggered when the enemy sees the player
  (set `self.CanSeePlayer` true)
  (set `self.TimeSincePlayerSeen` 0.0))

(event `self.ReceiveBeginPlay`
  (set `self.CanSeePlayer` false)
  (set `self.At Location` true)
  (set `self.CanAttack` true)
  ; Add all target locations to the array Possible Locations
  (bind _outactors (`GameplayStatics.GetAllActorsOfClass` "/Script/Engine.TargetPoint"))
  (for _array_element _outactors
    (`KismetArrayLibrary.Array_Add` (`self.PossibleLocations`) _array_element))
  (set `self.SpawnAnimation` true)
  (`KismetSystemLibrary.Delay` 2.0)
  (set `self.SpawnAnimation` false))

(event `self.ReceiveTick`
  (params (DeltaSeconds :type "Float (single-precision)"))
  (if (not (`self.SpawnAnimation`))
    (`|ExecutionSequence`
      (:`then_0`
        ; If the enemy can see the player, then check how long since the enemy last sawt the player. If > 2 seconds, pick a new location
        (if (`self.CanSeePlayer`)
          (set `self.CurrentTarget` (`GameplayStatics.GetPlayerController` 0))
          (set `self.TimeSincePlayerSeen` (+ (`self.TimeSincePlayerSeen`) DeltaSeconds))
          (if (> (`self.TimeSincePlayerSeen`) 2.0)
            ;; At Location is set to true to make sure the agent picks a new location
            (set `self.CanSeePlayer` false)
            (set `self.At Location` true))))
      (:`then_1`
        (if (`self.CanSeePlayer`)
          ; If the enemy can see the player, move towards them
          (set `self.CanAttack` true)
          (`|AIMoveTo` self (0.0 0.0 0.0) (`GameplayStatics.GetPlayerController` 0) 70.0
            (:`OnSuccess`
              ; If the enemy reaches the player, play the attack animation
              (if (`self.CanAttack`)
                (set `self.CanAttack` false)
                (`KismetSystemLibrary.Delay` 1.8)
                (set `self.CanAttack` true)
                (`KismetSystemLibrary.PrintString` "Hello"))))
          (else
            (if (`self.At Location`)
              ; If the enemy has reached the target location, pick a location from possible locations to move tto (Note, this can pick the same location the enemy has just reached, but this will eventually rroll a different location)
              (set `self.CurrentTarget` (`KismetArrayLibrary.Array_Random` (`self.PossibleLocations`)))
              (set `self.At Location` false))
            ; Move towards target location
            (`|AIMoveTo` self (0.0 0.0 0.0) (`self.CurrentTarget`)
              (:`OnSuccess`
                (set `self.At Location` true)))))))))

(event `Follow Player`
  ; Comment
  (if (`self.CanSeePlayer`)
    (`|AIMoveTo` self (0.0 0.0 0.0) (`GameplayStatics.GetPlayerCharacter` 0))
    (else
      (set `self.CanSeePlayer` false))))

(fn `UserConstructionScript`)